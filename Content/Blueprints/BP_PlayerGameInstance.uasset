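; BP_PlayerGameInstance is a game instance that makes player preferences save data available when the game starts.
; On Init it checks for the save slot and loads an existing save as BP_PlayerPreferences into SaveGameData.
; If no save exists, it creates a new BP_PlayerPreferences object, stores it in SaveGameData and writes it to the slot immediately.
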(event `self.ReceiveInit`
  (bind _returnvalue (`GameplayStatics.DoesSaveGameExist` (`self.SaveSlotName`)))
  (if _returnvalue
    (bind _returnvalue_2 (`GameplayStatics.LoadGameFromSlot` (`self.SaveSlotName`)))
    (bind _asbp_player_preferences (cast `/Game/Blueprints/BP_PlayerPreferences` _returnvalue_2))
    (set `self.SaveGameData` _asbp_player_preferences)
    (else
      (bind _returnvalue_3 (`GameplayStatics.CreateSaveGameObject` "/Game/Blueprints/BP_PlayerPreferences.BP_PlayerPreferences_C"))
      (bind _output_get (set `self.SaveGameData` _returnvalue_3))
      (`GameplayStatics.SaveGameToSlot` _output_get (`self.SaveSlotName`)))))